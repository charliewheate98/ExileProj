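; Interactive object Blueprint that responds to player interaction with a placeholder "Hello" debug print.
; Every Tick it casts the player character to FirstPersonCharacter and, while Interacting is set, prints if that character's CheckInteraction returns true.
; A radius-based distance check between the InteractiveObject component and the player exists but is disconnected and never runs.
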(event `self.ReceiveTick`
  (params (DeltaSeconds :type "Float (single-precision)"))
  ;[1 1 1] Look Check
  (bind _asfirst_person_character (cast `/Game/FirstPersonBP/Blueprints/FirstPersonCharacter` (`GameplayStatics.GetPlayerCharacter` 0)))
  (if (`/Game/FirstPersonBP/Blueprints/FirstPersonCharacter.Interacting` _asfirst_person_character)
    (bind _ishit (`/Game/FirstPersonBP/Blueprints/FirstPersonCharacter.Check Interaction` _asfirst_person_character))
    (if _ishit
      (`KismetSystemLibrary.PrintString` "Hello"))))

(fn `UserConstructionScript`)